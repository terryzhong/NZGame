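; Red variant of the zombie tank AI character that connects the character to its animation Blueprint.
; On BeginPlay it casts and caches the mesh's AnimBP_ZombieTank instance and switches on its wander flag.
; When hit effects play, it runs the parent's effects and then calls TakeHit on the cached anim instance.
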(event EventPlayTakeHitEffects
  (|CallParentFunction)
  (Default|TakeHit (Variables|Default|GetAnimBPZombieTank)))

(event EventBeginPlay
  (bind _asanim_bp_zombie_tank (Utilities|Casting|CastToAnimBP_ZombieTank (Components|SkeletalMesh|GetAnimInstance (Variables|Character|GetMesh))))
  (bind _output_get (Variables|Default|SetAnimBPZombieTank _asanim_bp_zombie_tank))
  (Variables|/Game/AICharacters/ZombieTank/Animations/AnimBP_ZombieTank.AnimBP_ZombieTank_C|SetIsWander _output_get true))

(event EventActorBeginOverlap
  (params (OtherActor :type Actor%20Object%20Reference)))

(event EventTick
  (params (DeltaSeconds :type Float%20%28single-precision%29)))

(fn ConstructionScript
  (|CallParentFunction))